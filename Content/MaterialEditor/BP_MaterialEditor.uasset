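; In-game material editor actor that previews a chosen static mesh and edits its material at runtime through WBP_MaterialEditor, shown with Right Ctrl.
; Widget events drive mesh, material, scale, visibility and scalar, vector or texture parameters on a dynamic material instance.
; GetPackageName converts DeadByDaylight content file paths to /Game/ paths for blocking asset loads.
; Tick places the actor on the player character or at the position saved on mesh change.
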(event `self.ReceiveBeginPlay`
  (bind _returnvalue (`|CreateWidget` "/Game/MaterialEditor/WBP_MaterialEditor.WBP_MaterialEditor_C"))
  (bind _output_get (set `self.WidgetRef` _returnvalue))
  (`UserWidget.AddToViewport` _output_get 0)
  (`Widget.SetVisibility` (`self.WidgetRef`) "Collapsed")
  (add `/Game/MaterialEditor/WBP_MaterialEditor.OnMeshChanged` (`self.WidgetRef`) (delegate `OnMeshChanged_Event`))
  (add `/Game/MaterialEditor/WBP_MaterialEditor.OnFollowLocalCharacterChecked` (`self.WidgetRef`) (delegate `OnFollowLocalCharacterChecked_Event`))
  (add `/Game/MaterialEditor/WBP_MaterialEditor.OnMaterialChanged` (`self.WidgetRef`) (delegate `OnMaterialChanged_Event`))
  (add `/Game/MaterialEditor/WBP_MaterialEditor.OnScaleApplied` (`self.WidgetRef`) (delegate `OnScaleApplied_Event`))
  (add `/Game/MaterialEditor/WBP_MaterialEditor.OnScalarParameterChanged` (`self.WidgetRef`) (delegate `OnScalarParameterChanged_Event`))
  (add `/Game/MaterialEditor/WBP_MaterialEditor.OnVectorParameterChanged` (`self.WidgetRef`) (delegate `OnVectorParameterChanged_Event`))
  (add `/Game/MaterialEditor/WBP_MaterialEditor.OnTextureParameterChanged` (`self.WidgetRef`) (delegate `OnTextureParameterChanged_Event`))
  (add `/Game/MaterialEditor/WBP_MaterialEditor.OnMeshVisibilityChanged` (`self.WidgetRef`) (delegate `OnMeshVisibilityChanged_Event`)))

(event `OnFollowLocalCharacterChecked_Event`
  (params (IsChecked :type Boolean))
  (`self.FollowLocalCharacter` IsChecked))

(event `OnMeshChanged_Event`
  (params (StaticMeshPath :type String))
  (`self.ChangeMesh` StaticMeshPath))

(event `OnMaterialChanged_Event`
  (params (MaterialPath :type String))
  (`self.ChangeMaterial` MaterialPath))

(event `OnScaleApplied_Event`
  (params (Scale :type "Float (double-precision)"))
  (`self.ApplyScale` Scale))

(event `OnScalarParameterChanged_Event`
  (params (ParameterName :type Name) (Value :type "Float (double-precision)"))
  (`self.SetScalarParameter` ParameterName Value))

(event `OnVectorParameterChanged_Event`
  (params (ParameterName :type Name) (Value :type "LinearColor Structure"))
  (`self.SetVectorParameter` ParameterName Value))

(event `OnTextureParameterChanged_Event`
  (params (ParameterName :type Name) (Value :type String))
  (`self.SetTextureParameter` ParameterName Value))

(event `OnMeshVisibilityChanged_Event`
  (params (IsVisible :type Boolean))
  (`self.SetMeshVisibility` IsVisible))

(event `self.ReceiveTick`
  (params (DeltaSeconds :type "Float (single-precision)"))
  (`|ExecutionSequence`
    (:`then_0`
      (`self.K2_SetActorTransform` (`KismetMathLibrary.MakeTransform` (`KismetMathLibrary.SelectVector` (.location (`self.GetTransform` (`GameplayStatics.GetPlayerCharacter` 0))) (.location (`self.OriginalPos`)) (`self.FollowCharacter`)) (.rotation (`self.GetTransform`)) (.scale (`self.GetTransform`)))))
    (:`then_1`
      (if (`PlayerController.WasInputKeyJustPressed` (`GameplayStatics.GetPlayerController` 0) "RightControl")
        (`Widget.SetVisibility` (`self.WidgetRef`) "Visible")
        (`WidgetBlueprintLibrary.SetInputMode_UIOnlyEx` (`GameplayStatics.GetPlayerController` 0) (`self.WidgetRef`))
        (set `PlayerController.bShowMouseCursor` true (`GameplayStatics.GetPlayerController` 0))))))

(fn `ApplyScale`
  (params (Scale :type "Float (double-precision)"))
  (`/Game/LoggingUtilities_OldHUD/BlueprintLoggingLibrary.PrintString` (`KismetTextLibrary.Conv_TextToString` (`|FormatText` "New scale: {sc}" Scale)))
  (`SceneComponent.SetRelativeScale3D` (`self.StaticMesh`) (`KismetMathLibrary.MakeVector` Scale Scale Scale)))

(fn `ChangeMaterial`
  (params (MeshPath :type String))
  (bind _returnvalue (`KismetSystemLibrary.LoadAsset_Blocking` (`KismetSystemLibrary.Conv_SoftObjPathToSoftObjRef` (`KismetSystemLibrary.MakeSoftObjectPath` (`self.GetPackageName` MeshPath)))))
  (bind _asmaterial_instance (cast `MaterialInstance` _returnvalue))
  (`PrimitiveComponent.SetMaterial` (`self.StaticMesh`) 0 _asmaterial_instance)
  (bind _returnvalue_2 (`PrimitiveComponent.CreateDynamicMaterialInstance` (`self.StaticMesh`) 0 null "None"))
  (set `self.DynamicMaterial` _returnvalue_2))

(fn `ChangeMesh`
  (params (MeshPath :type String))
  (bind _returnvalue (`KismetSystemLibrary.LoadAsset_Blocking` (`KismetSystemLibrary.Conv_SoftObjPathToSoftObjRef` (`KismetSystemLibrary.MakeSoftObjectPath` (`self.GetPackageName` MeshPath)))))
  (bind _asstatic_mesh (cast `StaticMesh` _returnvalue))
  (`StaticMeshComponent.SetStaticMesh` (`self.StaticMesh`) _asstatic_mesh)
  (bind _returnvalue_2 (`PrimitiveComponent.CreateDynamicMaterialInstance` (`self.StaticMesh`) 0 null "None"))
  (set `self.DynamicMaterial` _returnvalue_2)
  (set `self.OriginalPos` (`self.GetTransform` (`GameplayStatics.GetPlayerCharacter` 0))))

(fn `FollowLocalCharacter`
  (params (Follow :type Boolean))
  (set `self.FollowCharacter` Follow))

(fn `GetPackageName`
  (params (String :type String))
  (returns (PackageName :type String))
  (if (`KismetStringLibrary.StartsWith` String "/" "CaseSensitive")
    (return (`local.String`))
    (else
      (return (`KismetStringLibrary.Concat_StrStr` (`KismetStringLibrary.Concat_StrStr` (`KismetStringLibrary.Replace` (`KismetStringLibrary.Split` (`local.String`) "." "CaseSensitive" "FromEnd") "DeadByDaylight/Content/" "/Game/" "CaseSensitive") ".") (`KismetStringLibrary.Split` (`.RightS` (`KismetStringLibrary.Split` (`local.String`) "/" "CaseSensitive" "FromEnd")) "." "CaseSensitive"))))))

(fn `SetMeshVisibility`
  (params (IsVisible :type Boolean))
  (`SceneComponent.SetVisibility` (`self.StaticMesh`) IsVisible false))

(fn `SetScalarParameter`
  (params (ParameterName :type Name) (Value :type "Float (double-precision)"))
  (`MaterialInstanceDynamic.SetScalarParameterValue` (`self.DynamicMaterial`) ParameterName Value))

(fn `SetTextureParameter`
  (params (ParameterName :type Name) (Value :type String))
  (bind _returnvalue (`KismetSystemLibrary.LoadAsset_Blocking` (`KismetSystemLibrary.Conv_SoftObjPathToSoftObjRef` (`KismetSystemLibrary.MakeSoftObjectPath` (`self.GetPackageName` Value)))))
  (bind _astexture (cast `Texture` _returnvalue))
  (`MaterialInstanceDynamic.SetTextureParameterValue` (`self.DynamicMaterial`) (`local.ParameterName`) _astexture))

(fn `SetVectorParameter`
  (params (ParameterName :type Name) (Value :type "LinearColor Structure"))
  (`MaterialInstanceDynamic.SetVectorParameterValue` (`self.DynamicMaterial`) ParameterName Value))

(fn `UserConstructionScript`)